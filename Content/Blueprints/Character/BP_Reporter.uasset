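; Reporter character whose current mood sets its skeletal mesh and looping animation.
; SetCurrentMood looks up the mood in the MoodMeshes map, swaps the mesh and plays the paired animation directly on it, bypassing the Anim Blueprint.
; NextMood steps through the EMoods enum in order until a final mood.
; BeginPlay caches the BP_AimPamala anim instance, which these graphs never use afterward.
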(event EventBeginPlay
  (bind _asbp_aim_pamala (Utilities|Casting|CastToBP_AimPamala (Components|SkeletalMesh|GetAnimInstance (Variables|Character|GetMesh))))
  (Variables|Default|SetAs%20BP%20Aim%20Pamala _asbp_aim_pamala))

(event Collision|EventActorBeginOverlap
  (params (OtherActor :type Actor%20Object%20Reference)))

(event EventTick
  (params (DeltaSeconds :type Float%20%28single-precision%29)))

(fn ConstructionScript)

(fn SetCurrentMood
  (params (CurrentMood :type EMoods%20Enum :default "NewEnumerator0"))
  (bind _mesh (Variables|Character|GetMesh))
  (Variables|Default|SetCurrentMood CurrentMood)
  (Class|SkinnedMeshComponent|SetSkeletalMesh _mesh (.MoodSkeletalMesh (Utilities|Struct|BreakMoodStruct (.Value (Utilities|Map|Find (Variables|Default|GetMoodMeshes) (Variables|Default|GetCurrentMood))))) true)
  (Components|Animation|PlayAnimation _mesh (.Montage (Utilities|Struct|BreakMoodStruct (.Value (Utilities|Map|Find (Variables|Default|GetMoodMeshes) (Variables|Default|GetCurrentMood))))) true)
  (Audio|Components|Audio|Play _mesh true))

(fn GetCurrentMood
  (return (Variables|Default|GetCurrentMood)))

(fn NextMood
  (if (Utilities|Enum|NotEqual(Enum) (Variables|Default|GetCurrentMood) "NewEnumerator4")
    (CallFunction|SetCurrentMood (Utilities|Enum|ByteToEnumEMoods (+ (Variables|Default|GetCurrentMood) 1)))))