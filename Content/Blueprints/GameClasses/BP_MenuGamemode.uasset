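; BP_MenuGamemode is the game mode for menu levels, setting up the main menu when play begins.
; It creates WBP_MainMenu, adds it to the viewport, switches to UI-only input with the cursor shown, and plays the menu sound cue at the player pawn's location.
; If the current level is creditsMap, it tells the menu widget to show the credits.
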(event EventBeginPlay
  (bind _returnvalue (Game|GetPlayerController 0))
  (bind _returnvalue_2 (UserInterface|CreateWidget "/Game/Blueprints/UI/WBP_MainMenu.WBP_MainMenu_C"))
  (UserInterface|Viewport|AddtoViewport _returnvalue_2 0)
  (Input|SetInputModeUIOnly _returnvalue _returnvalue_2 "DoNotLock")
  (Variables|/Script/Engine.PlayerController|SetbShowMouseCursor _returnvalue true)
  (Audio|PlaySoundatLocation "/Game/AudioFiles/Designer/Music/Cue_MainMenu.Cue_MainMenu" (Transformation|GetActorLocation (Game|Player|GetPlayerPawn 0)) "0, 0, 0" 1.0 1.0 0.0 0 0 0)
  (bind _returnvalue_3 (Game|GetCurrentLevelName true))
  (if (Utilities|Enum|Equal(Enum) _returnvalue_3 "creditsMap")
    (Default|SetCreditsVisibleon _returnvalue_2)))

(event EventTick
  (params (DeltaSeconds :type Float%20%28single-precision%29)))

(fn ConstructionScript)